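; BP_DatasetGenerator automatically builds a synthetic image dataset of in-world ads for detection and segmentation training.
; After collecting BP_AdTarget and BP_CameraPoint actors, it loops through frames, randomizing camera point, FOV and weather before saving a capture.
; It projects ad corners to 1280x720 pixels, filtering by screen bounds, box size and center line-trace occlusion.
; It saves normalized YOLO-style box labels, plus four-corner polygon labels for fully on-screen ads.
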(event Custom|GenerateLabelsForCurrentFrame
  (bind _rendercameraref (Variables|Default|GetRenderCameraRef))
  (Variables|Default|SetCurrentLabelText "")
  (Variables|Default|SetCurrentSegmentationLabelText "")
  (Variables|Default|SetVisibleAdCount 0)
  (for _array_element (Variables|Default|GetAdTargets)
    (Utilities|IsValid _array_element
      (:Is%20Valid
        (bind (_corner1 _corner2 _corner3 _corner4) (Default|GetAdFaceCornersWorld _array_element))
        (bind (_pixelposition _isinfront) (Default|ProjectWorldtoImagePoint _rendercameraref _corner1))
        (bind (_pixelposition_2 _isinfront_2) (Default|ProjectWorldtoImagePoint _rendercameraref _corner2))
        (bind (_pixelposition_3 _isinfront_3) (Default|ProjectWorldtoImagePoint _rendercameraref _corner3))
        (bind (_pixelposition_4 _isinfront_4) (Default|ProjectWorldtoImagePoint _rendercameraref _corner4))
        (if (and (and _isinfront _isinfront_2) (and _isinfront_3 _isinfront_4))
          (if (and (and (< (Math|Float|Min(Float) (Math|Float|Min(Float) (.X (Math|Vector2D|BreakVector2D _pixelposition)) (.X (Math|Vector2D|BreakVector2D _pixelposition_2))) (Math|Float|Min(Float) (.X (Math|Vector2D|BreakVector2D _pixelposition_3)) (.X (Math|Vector2D|BreakVector2D _pixelposition_4)))) 1.28e+03) (> (Math|Float|Max(Float) (Math|Float|Max(Float) (.X (Math|Vector2D|BreakVector2D _pixelposition)) (.X (Math|Vector2D|BreakVector2D _pixelposition_2))) (Math|Float|Max(Float) (.X (Math|Vector2D|BreakVector2D _pixelposition_3)) (.X (Math|Vector2D|BreakVector2D _pixelposition_4)))) 0.0)) (and (< (Math|Float|Min(Float) (Math|Float|Min(Float) (.Y (Math|Vector2D|BreakVector2D _pixelposition)) (.Y (Math|Vector2D|BreakVector2D _pixelposition_2))) (Math|Float|Min(Float) (.Y (Math|Vector2D|BreakVector2D _pixelposition_3)) (.Y (Math|Vector2D|BreakVector2D _pixelposition_4)))) 7.2e+02) (> (Math|Float|Max(Float) (Math|Float|Max(Float) (.Y (Math|Vector2D|BreakVector2D _pixelposition)) (.Y (Math|Vector2D|BreakVector2D _pixelposition_2))) (Math|Float|Max(Float) (.Y (Math|Vector2D|BreakVector2D _pixelposition_3)) (.Y (Math|Vector2D|BreakVector2D _pixelposition_4)))) 0.0)))
            (bind _isvisible (CallFunction|IsAdCenterVisible _array_element))
            (if _isvisible
              (if (and (>= (- (Math|Float|Max(Float) (Math|Float|Max(Float) (.X (Math|Vector2D|BreakVector2D _pixelposition)) (.X (Math|Vector2D|BreakVector2D _pixelposition_2))) (Math|Float|Max(Float) (.X (Math|Vector2D|BreakVector2D _pixelposition_3)) (.X (Math|Vector2D|BreakVector2D _pixelposition_4)))) (Math|Float|Min(Float) (Math|Float|Min(Float) (.X (Math|Vector2D|BreakVector2D _pixelposition)) (.X (Math|Vector2D|BreakVector2D _pixelposition_2))) (Math|Float|Min(Float) (.X (Math|Vector2D|BreakVector2D _pixelposition_3)) (.X (Math|Vector2D|BreakVector2D _pixelposition_4))))) (Variables|Default|GetMinBoxWidth)) (>= (- (Math|Float|Max(Float) (Math|Float|Max(Float) (.Y (Math|Vector2D|BreakVector2D _pixelposition)) (.Y (Math|Vector2D|BreakVector2D _pixelposition_2))) (Math|Float|Max(Float) (.Y (Math|Vector2D|BreakVector2D _pixelposition_3)) (.Y (Math|Vector2D|BreakVector2D _pixelposition_4)))) (Math|Float|Min(Float) (Math|Float|Min(Float) (.Y (Math|Vector2D|BreakVector2D _pixelposition)) (.Y (Math|Vector2D|BreakVector2D _pixelposition_2))) (Math|Float|Min(Float) (.Y (Math|Vector2D|BreakVector2D _pixelposition_3)) (.Y (Math|Vector2D|BreakVector2D _pixelposition_4))))) (Variables|Default|GetMinBoxHeight)))
                (Variables|Default|SetVisibleAdCount (+ (Variables|Default|GetVisibleAdCount) 1))
                (Variables|Default|SetCurrentLabelText (Utilities|String|Append (Variables|Default|GetCurrentLabelText) (Utilities|String|Append (Utilities|String|ToString(Integer) (Variables|/Game/Synthetic_Dataset/Blueprints/BP_AdTarget.BP_AdTarget_C|GetClassID _array_element)) " " (Utilities|String|ToString(Float) (/ (/ (+ (Math|Float|Clamp(Float) (Math|Float|Min(Float) (Math|Float|Min(Float) (.X (Math|Vector2D|BreakVector2D _pixelposition)) (.X (Math|Vector2D|BreakVector2D _pixelposition_2))) (Math|Float|Min(Float) (.X (Math|Vector2D|BreakVector2D _pixelposition_3)) (.X (Math|Vector2D|BreakVector2D _pixelposition_4)))) 0.0 1.28e+03) (Math|Float|Clamp(Float) (Math|Float|Max(Float) (Math|Float|Max(Float) (.X (Math|Vector2D|BreakVector2D _pixelposition)) (.X (Math|Vector2D|BreakVector2D _pixelposition_2))) (Math|Float|Max(Float) (.X (Math|Vector2D|BreakVector2D _pixelposition_3)) (.X (Math|Vector2D|BreakVector2D _pixelposition_4)))) 0.0 1.28e+03)) 2.0) 1.28e+03)) " " (Utilities|String|ToString(Float) (/ (/ (+ (Math|Float|Clamp(Float) (Math|Float|Min(Float) (Math|Float|Min(Float) (.Y (Math|Vector2D|BreakVector2D _pixelposition)) (.Y (Math|Vector2D|BreakVector2D _pixelposition_2))) (Math|Float|Min(Float) (.Y (Math|Vector2D|BreakVector2D _pixelposition_3)) (.Y (Math|Vector2D|BreakVector2D _pixelposition_4)))) 0.0 7.2e+02) (Math|Float|Clamp(Float) (Math|Float|Max(Float) (Math|Float|Max(Float) (.Y (Math|Vector2D|BreakVector2D _pixelposition)) (.Y (Math|Vector2D|BreakVector2D _pixelposition_2))) (Math|Float|Max(Float) (.Y (Math|Vector2D|BreakVector2D _pixelposition_3)) (.Y (Math|Vector2D|BreakVector2D _pixelposition_4)))) 0.0 7.2e+02)) 2.0) 7.2e+02)) " " (Utilities|String|ToString(Float) (/ (- (Math|Float|Clamp(Float) (Math|Float|Max(Float) (Math|Float|Max(Float) (.X (Math|Vector2D|BreakVector2D _pixelposition)) (.X (Math|Vector2D|BreakVector2D _pixelposition_2))) (Math|Float|Max(Float) (.X (Math|Vector2D|BreakVector2D _pixelposition_3)) (.X (Math|Vector2D|BreakVector2D _pixelposition_4)))) 0.0 1.28e+03) (Math|Float|Clamp(Float) (Math|Float|Min(Float) (Math|Float|Min(Float) (.X (Math|Vector2D|BreakVector2D _pixelposition)) (.X (Math|Vector2D|BreakVector2D _pixelposition_2))) (Math|Float|Min(Float) (.X (Math|Vector2D|BreakVector2D _pixelposition_3)) (.X (Math|Vector2D|BreakVector2D _pixelposition_4)))) 0.0 1.28e+03)) 1.28e+03)) " " (Utilities|String|ToString(Float) (/ (- (Math|Float|Clamp(Float) (Math|Float|Max(Float) (Math|Float|Max(Float) (.Y (Math|Vector2D|BreakVector2D _pixelposition)) (.Y (Math|Vector2D|BreakVector2D _pixelposition_2))) (Math|Float|Max(Float) (.Y (Math|Vector2D|BreakVector2D _pixelposition_3)) (.Y (Math|Vector2D|BreakVector2D _pixelposition_4)))) 0.0 7.2e+02) (Math|Float|Clamp(Float) (Math|Float|Min(Float) (Math|Float|Min(Float) (.Y (Math|Vector2D|BreakVector2D _pixelposition)) (.Y (Math|Vector2D|BreakVector2D _pixelposition_2))) (Math|Float|Min(Float) (.Y (Math|Vector2D|BreakVector2D _pixelposition_3)) (.Y (Math|Vector2D|BreakVector2D _pixelposition_4)))) 0.0 7.2e+02)) 7.2e+02)) " 
")))
                (if (|CollapseGraph (.X (Math|Vector2D|BreakVector2D _pixelposition)) (.X (Math|Vector2D|BreakVector2D _pixelposition)) (.Y (Math|Vector2D|BreakVector2D _pixelposition)) (.Y (Math|Vector2D|BreakVector2D _pixelposition)) (.X (Math|Vector2D|BreakVector2D _pixelposition_2)) (.X (Math|Vector2D|BreakVector2D _pixelposition_2)) (.Y (Math|Vector2D|BreakVector2D _pixelposition_2)) (.Y (Math|Vector2D|BreakVector2D _pixelposition_2)) (.X (Math|Vector2D|BreakVector2D _pixelposition_3)) (.X (Math|Vector2D|BreakVector2D _pixelposition_3)) (.Y (Math|Vector2D|BreakVector2D _pixelposition_3)) (.Y (Math|Vector2D|BreakVector2D _pixelposition_3)) (.X (Math|Vector2D|BreakVector2D _pixelposition_4)) (.X (Math|Vector2D|BreakVector2D _pixelposition_4)) (.Y (Math|Vector2D|BreakVector2D _pixelposition_4)) (.Y (Math|Vector2D|BreakVector2D _pixelposition_4)))
                  (Variables|Default|SetCurrentSegmentationLabelText (Utilities|String|Append (Variables|Default|GetCurrentSegmentationLabelText) (Utilities|String|Append (Utilities|String|ToString(Integer) (Variables|/Game/Synthetic_Dataset/Blueprints/BP_AdTarget.BP_AdTarget_C|GetClassID _array_element)) " " (Utilities|String|ToString(Float) (.ReturnValue (|NormalizingValues (.X (Math|Vector2D|BreakVector2D _pixelposition)) (.Y (Math|Vector2D|BreakVector2D _pixelposition)) (.X (Math|Vector2D|BreakVector2D _pixelposition_2)) (.Y (Math|Vector2D|BreakVector2D _pixelposition_2)) (.X (Math|Vector2D|BreakVector2D _pixelposition_3)) (.Y (Math|Vector2D|BreakVector2D _pixelposition_3)) (.X (Math|Vector2D|BreakVector2D _pixelposition_4)) (.Y (Math|Vector2D|BreakVector2D _pixelposition_4))))) " " (Utilities|String|ToString(Float) (.ReturnValue2 (|NormalizingValues (.X (Math|Vector2D|BreakVector2D _pixelposition)) (.Y (Math|Vector2D|BreakVector2D _pixelposition)) (.X (Math|Vector2D|BreakVector2D _pixelposition_2)) (.Y (Math|Vector2D|BreakVector2D _pixelposition_2)) (.X (Math|Vector2D|BreakVector2D _pixelposition_3)) (.Y (Math|Vector2D|BreakVector2D _pixelposition_3)) (.X (Math|Vector2D|BreakVector2D _pixelposition_4)) (.Y (Math|Vector2D|BreakVector2D _pixelposition_4))))) " " (Utilities|String|ToString(Float) (.ReturnValue3 (|NormalizingValues (.X (Math|Vector2D|BreakVector2D _pixelposition)) (.Y (Math|Vector2D|BreakVector2D _pixelposition)) (.X (Math|Vector2D|BreakVector2D _pixelposition_2)) (.Y (Math|Vector2D|BreakVector2D _pixelposition_2)) (.X (Math|Vector2D|BreakVector2D _pixelposition_3)) (.Y (Math|Vector2D|BreakVector2D _pixelposition_3)) (.X (Math|Vector2D|BreakVector2D _pixelposition_4)) (.Y (Math|Vector2D|BreakVector2D _pixelposition_4))))) " " (Utilities|String|ToString(Float) (.ReturnValue4 (|NormalizingValues (.X (Math|Vector2D|BreakVector2D _pixelposition)) (.Y (Math|Vector2D|BreakVector2D _pixelposition)) (.X (Math|Vector2D|BreakVector2D _pixelposition_2)) (.Y (Math|Vector2D|BreakVector2D _pixelposition_2)) (.X (Math|Vector2D|BreakVector2D _pixelposition_3)) (.Y (Math|Vector2D|BreakVector2D _pixelposition_3)) (.X (Math|Vector2D|BreakVector2D _pixelposition_4)) (.Y (Math|Vector2D|BreakVector2D _pixelposition_4))))) " " (Utilities|String|ToString(Float) (.ReturnValue5 (|NormalizingValues (.X (Math|Vector2D|BreakVector2D _pixelposition)) (.Y (Math|Vector2D|BreakVector2D _pixelposition)) (.X (Math|Vector2D|BreakVector2D _pixelposition_2)) (.Y (Math|Vector2D|BreakVector2D _pixelposition_2)) (.X (Math|Vector2D|BreakVector2D _pixelposition_3)) (.Y (Math|Vector2D|BreakVector2D _pixelposition_3)) (.X (Math|Vector2D|BreakVector2D _pixelposition_4)) (.Y (Math|Vector2D|BreakVector2D _pixelposition_4))))) " " (Utilities|String|ToString(Float) (.ReturnValue6 (|NormalizingValues (.X (Math|Vector2D|BreakVector2D _pixelposition)) (.Y (Math|Vector2D|BreakVector2D _pixelposition)) (.X (Math|Vector2D|BreakVector2D _pixelposition_2)) (.Y (Math|Vector2D|BreakVector2D _pixelposition_2)) (.X (Math|Vector2D|BreakVector2D _pixelposition_3)) (.Y (Math|Vector2D|BreakVector2D _pixelposition_3)) (.X (Math|Vector2D|BreakVector2D _pixelposition_4)) (.Y (Math|Vector2D|BreakVector2D _pixelposition_4))))) " " (Utilities|String|ToString(Float) (.ReturnValue7 (|NormalizingValues (.X (Math|Vector2D|BreakVector2D _pixelposition)) (.Y (Math|Vector2D|BreakVector2D _pixelposition)) (.X (Math|Vector2D|BreakVector2D _pixelposition_2)) (.Y (Math|Vector2D|BreakVector2D _pixelposition_2)) (.X (Math|Vector2D|BreakVector2D _pixelposition_3)) (.Y (Math|Vector2D|BreakVector2D _pixelposition_3)) (.X (Math|Vector2D|BreakVector2D _pixelposition_4)) (.Y (Math|Vector2D|BreakVector2D _pixelposition_4))))) " " (Utilities|String|ToString(Float) (.ReturnValue8 (|NormalizingValues (.X (Math|Vector2D|BreakVector2D _pixelposition)) (.Y (Math|Vector2D|BreakVector2D _pixelposition)) (.X (Math|Vector2D|BreakVector2D _pixelposition_2)) (.Y (Math|Vector2D|BreakVector2D _pixelposition_2)) (.X (Math|Vector2D|BreakVector2D _pixelposition_3)) (.Y (Math|Vector2D|BreakVector2D _pixelposition_3)) (.X (Math|Vector2D|BreakVector2D _pixelposition_4)) (.Y (Math|Vector2D|BreakVector2D _pixelposition_4))))) " 
")))))))))))
  (Development|PrintString (Utilities|String|Append "Visible Ads In Image: " (Utilities|String|ToString(Integer) (Variables|Default|GetVisibleAdCount))))
  (Development|PrintString (Variables|Default|GetCurrentLabelText))
  (Development|PrintString (Variables|Default|GetCurrentSegmentationLabelText)))

(event Custom|SaveCurrentLabelFile
  (Class|DatasetFileUtils|SaveTexttoFile (Utilities|String|Append (Variables|Default|GetDetectionOutputFolder) "/" (Variables|Default|GetFrameBaseName) ".txt") (Variables|Default|GetCurrentLabelText))
  (Development|PrintString "Saved Detection Label File"))

(event Custom|SaveCurrentSegmentationLabelFile
  (Class|DatasetFileUtils|SaveTexttoFile (Utilities|String|Append (Variables|Default|GetSegmentationOutputFolder) "/" (Variables|Default|GetFrameBaseName) ".txt") (Variables|Default|GetCurrentSegmentationLabelText))
  (Development|PrintString "SavedSegmentationLabelFile"))

(event Custom|StartDatasetGeneration
  (Variables|Default|SetCurrentFrameIndex 5)
  (CallFunction|GenerateSingleFrame))

(event Custom|GenerateSingleFrame
  (CallFunction|MovetoRandomCameraPoint)
  (Game|Player|SetViewTargetwithBlend (Game|GetPlayerController 0) (Variables|Default|GetRenderCameraRef) 0.0 "VTBlend_Linear" 0.0 false)
  (Default|CollectFogActors (Variables|Default|GetWeatherControllerRef))
  (Default|ApplyRandomWeatherPreset (Variables|Default|GetWeatherControllerRef))
  (if (<= (Math|Random|RandomFloatinRange 0.0 1.0) 0.4)
    (Default|SetRainActive (Variables|Default|GetWeatherControllerRef) false))
  (Utilities|FlowControl|Delay 2.0)
  (CallFunction|GenerateLabelsforCurrentFrame)
  (Variables|Default|SetFrameBaseName (Utilities|String|Append "frame_" (Utilities|String|ToString(Integer) (Variables|Default|GetCurrentFrameIndex))))
  (Default|CaptureDatasetImage (Variables|Default|GetRenderCameraRef))
  (Utilities|FlowControl|Delay 0.2)
  (Default|SaveDatasetImage (Variables|Default|GetRenderCameraRef) (Variables|Default|GetImageOutputFolder) (Utilities|String|Append (Variables|Default|GetFrameBaseName) ".png"))
  (CallFunction|SaveCurrentLabelFile)
  (CallFunction|SaveCurrentSegmentationLabelFile)
  (bind _output_get (Variables|Default|SetCurrentFrameIndex (+ (Variables|Default|GetCurrentFrameIndex) 1)))
  (if (< _output_get (Variables|Default|GetTotalFramesToGenerate))
    (Utilities|FlowControl|Delay 3.0)
    (CallFunction|GenerateSingleFrame)
    (else
      (Development|PrintString "FinishedGeneratingDataset"))))

(event EventBeginPlay
  (CallFunction|CollectAdTargets)
  (CallFunction|CollectCameraPoints)
  (Utilities|FlowControl|Delay 2.0)
  (CallFunction|StartDatasetGeneration))

(event Collision|EventActorBeginOverlap
  (params (OtherActor :type Actor%20Object%20Reference)))

(event EventTick
  (params (DeltaSeconds :type Float%20%28single-precision%29)))

(fn ConstructionScript)

(fn CollectCameraPoints
  (Utilities|Array|Clear (Variables|Default|GetCameraPoints))
  (bind _outactors (Actor|GetAllActorsOfClass "/Game/Synthetic_Dataset/Blueprints/BP_CameraPoint.BP_CameraPoint_C"))
  (bind _output_get (Variables|Default|SetCameraPoints _outactors))
  (if (Variables|Default|GetDebugPrints)
    (Development|PrintString (Utilities|String|ToString(Integer) (Utilities|Array|Length _output_get)))))

(fn MovetoRandomCameraPoint
  (bind _camerapoints (Variables|Default|GetCameraPoints))
  (bind _rendercameraref (Variables|Default|GetRenderCameraRef))
  (bind _returnvalue (Utilities|Array|Length _camerapoints))
  (Utilities|IsValid (Variables|Default|GetRenderCameraRef)
    (:Is%20Valid
      (if (== _returnvalue 0)
        (Development|PrintString "NoCamerasFound")
        (else
          (bind _output_get (Variables|Default|SetCurrentCameraPoint (Utilities|Array|Get(acopy) (Variables|Default|GetCameraPoints) (Math|Random|RandomIntegerinRange 0 (- _returnvalue 1)))))
          (Transformation|SetActorLocation _rendercameraref (Transformation|GetActorLocation _output_get) false false)
          (Transformation|SetActorRotation _rendercameraref (Transformation|GetActorRotation _output_get))
          (Default|SetCameraFOV (Variables|Default|GetRenderCameraRef) (Math|Random|RandomFloatinRange (Variables|/Game/Synthetic_Dataset/Blueprints/BP_CameraPoint.BP_CameraPoint_C|GetMinFOV (Variables|Default|GetCurrentCameraPoint)) (Variables|/Game/Synthetic_Dataset/Blueprints/BP_CameraPoint.BP_CameraPoint_C|GetMaxFOV (Variables|Default|GetCurrentCameraPoint))))
          (Development|PrintString "MovedCameraAndSetFov"))))
    (:Is%20Not%20Valid
      (Development|PrintString "RenderCameraRef is not set"))))

(fn CollectAdTargets
  (Utilities|Array|Clear (Variables|Default|GetAdTargets))
  (bind _outactors (Actor|GetAllActorsOfClass "/Game/Synthetic_Dataset/Blueprints/BP_AdTarget.BP_AdTarget_C"))
  (bind _output_get (Variables|Default|SetAdTargets _outactors))
  (Development|PrintString (Utilities|String|ToString(Integer) (Utilities|Array|Length _output_get))))

(fn TestProjectFirstAd
  (bind _returnvalue (Class|WidgetLayoutLibrary|GetViewportScale))
  (bind _returnvalue_2 (Class|WidgetLayoutLibrary|GetViewportScale))
  (if (> (Utilities|Array|Length (Variables|Default|GetAdTargets)) 0)
    (bind (_corner1 _corner2 _corner3 _corner4) (Default|GetAdFaceCornersWorld (Variables|Default|GetDebugAdTargetRef)))
    (bind _pixelposition (Default|ProjectWorldtoImagePoint (Variables|Default|GetRenderCameraRef) _corner1))
    (bind _pixelposition_2 (Default|ProjectWorldtoImagePoint (Variables|Default|GetRenderCameraRef) _corner2))
    (bind _pixelposition_3 (Default|ProjectWorldtoImagePoint (Variables|Default|GetRenderCameraRef) _corner3))
    (bind _pixelposition_4 (Default|ProjectWorldtoImagePoint (Variables|Default|GetRenderCameraRef) _corner4))
    (Default|SetBox (Variables|Default|GetDebugBoxWidget) (Math|Vector2D|MakeVector2D (/ (Math|Float|Min(Float) (Math|Float|Min(Float) (.X (Math|Vector2D|BreakVector2D _pixelposition)) (.X (Math|Vector2D|BreakVector2D _pixelposition_2))) (Math|Float|Min(Float) (.X (Math|Vector2D|BreakVector2D _pixelposition_3)) (.X (Math|Vector2D|BreakVector2D _pixelposition_4)))) _returnvalue_2) (/ (Math|Float|Min(Float) (Math|Float|Min(Float) (.Y (Math|Vector2D|BreakVector2D _pixelposition)) (.Y (Math|Vector2D|BreakVector2D _pixelposition_2))) (Math|Float|Min(Float) (.Y (Math|Vector2D|BreakVector2D _pixelposition_3)) (.Y (Math|Vector2D|BreakVector2D _pixelposition_4)))) _returnvalue_2)) (Math|Vector2D|MakeVector2D (/ (- (Math|Float|Max(Float) (Math|Float|Max(Float) (.X (Math|Vector2D|BreakVector2D _pixelposition)) (.X (Math|Vector2D|BreakVector2D _pixelposition_2))) (Math|Float|Max(Float) (.X (Math|Vector2D|BreakVector2D _pixelposition_3)) (.X (Math|Vector2D|BreakVector2D _pixelposition_4)))) (Math|Float|Min(Float) (Math|Float|Min(Float) (.X (Math|Vector2D|BreakVector2D _pixelposition)) (.X (Math|Vector2D|BreakVector2D _pixelposition_2))) (Math|Float|Min(Float) (.X (Math|Vector2D|BreakVector2D _pixelposition_3)) (.X (Math|Vector2D|BreakVector2D _pixelposition_4))))) _returnvalue) (/ (- (Math|Float|Max(Float) (Math|Float|Max(Float) (.Y (Math|Vector2D|BreakVector2D _pixelposition)) (.Y (Math|Vector2D|BreakVector2D _pixelposition_2))) (Math|Float|Max(Float) (.Y (Math|Vector2D|BreakVector2D _pixelposition_3)) (.Y (Math|Vector2D|BreakVector2D _pixelposition_4)))) (Math|Float|Min(Float) (Math|Float|Min(Float) (.Y (Math|Vector2D|BreakVector2D _pixelposition)) (.Y (Math|Vector2D|BreakVector2D _pixelposition_2))) (Math|Float|Min(Float) (.Y (Math|Vector2D|BreakVector2D _pixelposition_3)) (.Y (Math|Vector2D|BreakVector2D _pixelposition_4))))) _returnvalue)))
    (else
      (Development|PrintString "NoAdTargetsFound"))))

(fn IsAdCenterVisible
  (params (AdTarget :type BP%20Ad%20Target%20Object%20Reference))
  (bind _adcenterworld (Default|GetAdCenterWorld AdTarget))
  (bind (_outhit _returnvalue) (Collision|LineTraceByChannel (Transformation|GetActorLocation (Variables|Default|GetRenderCameraRef)) _adcenterworld "TraceTypeQuery1" false (Utilities|Array|MakeArray (Variables|Default|GetRenderCameraRef) AdTarget) "None"))
  (if _returnvalue
    (return (<= (Math|Vector|Distance(Vector) (.Location (Collision|BreakHitResult _outhit)) _adcenterworld) (Variables|Default|GetOcclusionTolerance)))
    (else
      (return true))))
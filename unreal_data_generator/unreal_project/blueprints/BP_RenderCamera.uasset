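; Camera actor for synthetic dataset generation that renders images through a scene capture and exports them from a render target to disk.
; SetCameraFOV keeps the view camera, capture component and stored FOV in sync, and SetRainActive toggles a rain effect.
; ProjectWorldToImagePoint does manual pinhole projection from the capture's axes, FOV and image size, returning pixel coordinates and an in-front flag.
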(event EventBeginPlay)

(event Collision|EventActorBeginOverlap
  (params (OtherActor :type Actor%20Object%20Reference)))

(event EventTick
  (params (DeltaSeconds :type Float%20%28single-precision%29)))

(fn ConstructionScript)

(fn SetCameraFOV
  (params (NewFOV :type Float%20%28double-precision%29))
  (Camera|SetFieldOfView (Variables|Default|GetRenderCamera) NewFOV)
  (Variables|/Script/Engine.SceneCaptureComponent2D|SetFOVAngle (Variables|Default|GetDatasetCapture) NewFOV)
  (Variables|Default|SetCurrentFOV NewFOV))

(fn SetRainActive
  (params (Active :type Boolean))
  (if Active
    (Rendering|SetVisibility (Variables|Default|GetRainFX) true false)
    (Components|Activation|SetActive (Variables|Default|GetRainFX) true false)
    (else
      (Components|Activation|SetActive (Variables|Default|GetRainFX) false false)
      (Rendering|SetVisibility (Variables|Default|GetRainFX) false false))))

(fn CaptureDatasetImage
  (Rendering|SceneCapture|CaptureScene (Variables|Default|GetDatasetCapture) :!class /Script/Engine.SceneCaptureComponent2D))

(fn GetImageSize
  (return (Variables|Default|GetImageWidth) (Variables|Default|GetImageHeight)))

(fn SaveDatasetImage
  (params (FilePath :type String) (FileName :type String))
  (Rendering|ExportRenderTarget "/Game/Synthetic_Dataset/RenderTargets/RT_DatasetCapture.RT_DatasetCapture" FilePath FileName))

(fn ProjectWorldtoImagePoint
  (params (WorldLocation :type Vector))
  (bind _datasetcapture (Variables|Default|GetDatasetCapture))
  (bind _currentfov (Variables|Default|GetCurrentFOV))
  (bind _imagewidth (Variables|Default|GetImageWidth))
  (bind _datasetcapture_2 (Variables|Default|GetDatasetCapture))
  (bind _returnvalue (Math|Vector|GetForwardVector _datasetcapture))
  (bind _returnvalue_2 (Transformation|GetWorldLocation _datasetcapture_2))
  (bind _returnvalue_3 (Math|Conversions|ToFloat(Integer) _imagewidth))
  (bind _returnvalue_4 (* _currentfov 0.5))
  (bind _returnvalue_5 (Math|Trig|DegreesToRadians _returnvalue_4))
  (bind _returnvalue_6 (- WorldLocation _returnvalue_2))
  (bind _returnvalue_7 (* _returnvalue_3 0.5))
  (bind _returnvalue_8 (Math|Vector|DotProduct _returnvalue_6 _returnvalue))
  (bind _returnvalue_9 (Math|Trig|Tan(Radians) _returnvalue_5))
  (bind _returnvalue_10 (/ _returnvalue_7 _returnvalue_9))
  (return (Math|Vector2D|MakeVector2D (+ (* (Math|Conversions|ToFloat(Integer) (Variables|Default|GetImageWidth)) 0.5) (* _returnvalue_10 (/ (Math|Vector|DotProduct _returnvalue_6 (Math|Vector|GetRightVector _datasetcapture)) _returnvalue_8))) (- (* (Math|Conversions|ToFloat(Integer) (Variables|Default|GetImageHeight)) 0.5) (* (/ (Math|Vector|DotProduct _returnvalue_6 (Math|Vector|GetUpVector _datasetcapture)) _returnvalue_8) _returnvalue_10))) (> _returnvalue_8 1.0)))
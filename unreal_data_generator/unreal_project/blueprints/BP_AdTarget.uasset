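; BP_AdTarget is an ad target actor in the data generator that exposes the world-space geometry of an ad face, defined by its LabelBox component.
; GetAdFaceCornersWorld transforms four corners on the box's local XY mid-plane (Z=0) to world space, using unscaled extents so the component transform supplies the scale.
; GetAdCenterWorld returns the box's world location.
; The event graph and construction script contain no logic.
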(event EventBeginPlay)

(event Collision|EventActorBeginOverlap
  (params (OtherActor :type Actor%20Object%20Reference)))

(event EventTick
  (params (DeltaSeconds :type Float%20%28single-precision%29)))

(fn ConstructionScript)

(fn GetAdFaceCornersWorld
  (bind _labelbox (Variables|Default|GetLabelBox))
  (bind _labelbox_2 (Variables|Default|GetLabelBox))
  (bind _returnvalue (Transformation|GetWorldTransform _labelbox_2))
  (bind _returnvalue_2 (Components|Box|GetUnscaledBoxExtent _labelbox))
  (bind (_x _y) (Math|Vector|BreakVector _returnvalue_2))
  (bind _returnvalue_3 (* _x -1.0))
  (bind _returnvalue_4 (* _y -1.0))
  (return (Math|Transform|TransformLocation _returnvalue (Math|Vector|MakeVector _returnvalue_3 _returnvalue_4 0.0)) (Math|Transform|TransformLocation _returnvalue (Math|Vector|MakeVector _x _returnvalue_4 0.0)) (Math|Transform|TransformLocation _returnvalue (Math|Vector|MakeVector _x _y 0.0)) (Math|Transform|TransformLocation _returnvalue (Math|Vector|MakeVector _returnvalue_3 _y 0.0))))

(fn GetAdCenterWorld
  (return (Transformation|GetWorldLocation (Variables|Default|GetLabelBox))))